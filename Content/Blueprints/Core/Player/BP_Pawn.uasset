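; BP_Pawn is a player camera pawn that pans across the horizontal plane and zooms via a spring arm.
; Move and zoom input actions adjust a desired position and a clamped desired arm length, both seeded from the starting state on BeginPlay.
; Tick interpolates the actor location and spring arm length toward those targets for smoothed camera motion.
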(event `self.ReceiveBeginPlay`
  (set `self.Camera_pos_desired` (`self.K2_GetActorLocation`))
  (set `self.Zoom_desired` (`SpringArmComponent.TargetArmLength` (`self.SpringArm`))))

(event `self.ReceiveTick`
  (params (DeltaSeconds :type "Float (single-precision)"))
  (bind _springarm (`self.SpringArm`))
  (set `SpringArmComponent.TargetArmLength` (`KismetMathLibrary.FInterpTo` (`SpringArmComponent.TargetArmLength` _springarm) (`self.Zoom_desired`) DeltaSeconds 2.0) _springarm)
  (`self.K2_SetActorLocation` (`KismetMathLibrary.VInterpTo` (`self.K2_GetActorLocation`) (`self.Camera_pos_desired`) DeltaSeconds)))

(event `EnhancedInput|/Game/Blueprints/Core/Inputs/Input_camera_zoom`
  (params (ActionValue :type "Float (double-precision)") (ElapsedSeconds :type "Float (double-precision)") (TriggeredSeconds :type "Float (double-precision)") (InputAction :type "InputAction Object Reference" :default "/Game/Blueprints/Core/Inputs/Input_camera_zoom.Input_camera_zoom"))
  (:`Triggered`
    (set `self.Zoom_desired` (`KismetMathLibrary.FClamp` (+ (`self.Zoom_desired`) (* 20.0 ActionValue)) 100.0 2000.0))))

(event `EnhancedInput|/Game/Blueprints/Core/Inputs/Input_camera_move`
  (params (ActionValue :type "Vector2D Structure") (ElapsedSeconds :type "Float (double-precision)") (TriggeredSeconds :type "Float (double-precision)") (InputAction :type "InputAction Object Reference" :default "/Game/Blueprints/Core/Inputs/Input_camera_move.Input_camera_move"))
  (bind (_x _y) (`KismetMathLibrary.BreakVector2D` ActionValue))
  (:`Triggered`
    (set `self.Camera_pos_desired` (+ (`self.Camera_pos_desired`) (`KismetMathLibrary.MakeVector` (* 10.0 _x) (* 10.0 _y))))))

(fn `UserConstructionScript`)